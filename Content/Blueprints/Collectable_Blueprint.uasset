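; Collectable pickup that counts toward the player's collection and prompts islands to check whether they can unlock.
; On overlap with BP_Character, it calls CollectCollectible, then calls TryUnlock on BP_Island actors, with DestroyActor inside that loop.
; The Move timeline, given a random value at BeginPlay, animates the mesh's relative location, alternating forward and reverse through a delayed IsLooped toggle.
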(event EventBeginPlay
  (bind _moving (Timeline|Move Play)
    (:Update
      (Transformation|SetRelativeLocation (Variables|Default|GetStaticMeshComponent1) _moving false false)
      (Utilities|FlowControl|Delay 0.6)
      (if (Variables|Default|GetIsLooped)
        (Variables|Default|SetIsLooped false)
        (Timeline|Move Reverse)
        (else
          (Variables|Default|SetIsLooped true)
          (Timeline|Move Play))))))

(event Collision|EventActorBeginOverlap
  (params (OtherActor :type Actor%20Object%20Reference))
  ;[1 1 1] On Collecting the Collectible
  (bind _asbp_character (Utilities|Casting|CastToBP_Character OtherActor))
  (Default|CollectCollectible _asbp_character)
  (bind _outactors (Actor|GetAllActorsOfClass "/Game/Blueprints/BP_Island.BP_Island_C"))
  (for _array_element _outactors
    (Default|TryUnlock _array_element)
    (Actor|DestroyActor)))

(fn ConstructionScript)