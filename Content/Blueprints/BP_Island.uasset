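; BP_Island is an island Blueprint that moves into place when the player has found enough collectibles.
; TryUnlock reads CollectiblesFound from the player's BP_Character and calls Float if the island is not Unlocked and the count exactly equals UnlockQuota.
; Float moves the Island actor to FinalPosition in a single swept SetActorLocation.
; ItemCollected has no effect, and nothing shown sets Unlocked.
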(fn ConstructionScript)

(fn Float
  (Transformation|SetActorLocation (Variables|Default|GetIsland) (Variables|Default|GetFinalPosition) true false))

(fn ItemCollected
  (Utilities|Array|ForEachLoopwithBreak 0))

(fn TryUnlock
  (bind _asbp_character (Utilities|Casting|CastToBP_Character (Game|GetPlayerCharacter 0)))
  ;[1 1 1] Unlock the island
  (if (and (not (Variables|Default|GetUnlocked)) (== (Variables|/Game/Blueprints/BP_Character.BP_Character_C|GetCollectiblesFound _asbp_character) (Variables|Default|GetUnlockQuota)))
    (CallFunction|Float)))